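; Cart spawner that populates CartSpline paths with carts once the player's MotionControllerPawn has at least 50 points.
; A looping two-second timer gathers every CartSpline and triggers a spawn pass whenever fewer than four BabyCarts exist.
; Each pass spaces every spline's CartsOnSpline count evenly by distance, cycles through its Spawnables, and hands each cart its spline, distance and default controller.
; AI movement and randomisation nodes are unwired leftovers.
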(event `self.ReceiveBeginPlay`
  (`KismetSystemLibrary.K2_SetTimer` null "SpawnCart" 2.0 true))

(event `SpawnCart`
  (bind _asmotion_controller_pawn (cast `/Game/VirtualRealityBP/Blueprints/MotionControllerPawn` (`GameplayStatics.GetPlayerPawn` 0)))
  (if (>= (`/Game/VirtualRealityBP/Blueprints/MotionControllerPawn.Points` _asmotion_controller_pawn) 50)
    (bind _outactors (`GameplayStatics.GetAllActorsOfClass` "/Game/Blueprints/CartSpline.CartSpline_C"))
    ;[1 1 1] Check for cart amount and spawns another
    (set `self.SplineRef` _outactors)
    (bind _outactors_2 (`GameplayStatics.GetAllActorsOfClass` "/Game/Blueprints/BabyCarts.BabyCarts_C"))
    (if (< (`KismetArrayLibrary.Array_Length` _outactors_2) 4)
      (`self.SpawnCartOnSpline`))))

(event `MoveToPoint`)

(fn `SpawnCartOnSpline`
  (locals (CurrentSpline :type "/Game/Blueprints/CartSpline Object Reference") (CurrentSplineDistance :type "Float (double-precision)") (Division :type "Float (double-precision)") (Index :type Integer))
  (bind _index (`local.Index`))
  (bind _currentsplinedistance (`local.CurrentSplineDistance`))
  (bind _spline (`/Game/Blueprints/CartSpline.Spline` (`local.CurrentSpline`)))
  (bind _spawnables (`/Game/Blueprints/CartSpline.Spawnables` (`local.CurrentSpline`)))
  (for _array_element (`self.SplineRef`)
    (bind _output_get (set `local.CurrentSpline` _array_element))
    (bind _cartsonspline (`/Game/Blueprints/CartSpline.CartsOnSpline` _output_get))
    (set `local.Division` (/ (`SplineComponent.GetSplineLength` (`/Game/Blueprints/CartSpline.Spline` _output_get)) (`KismetMathLibrary.Conv_IntToDouble` _cartsonspline)))
    (for _ (range 1 (+ _cartsonspline 1))
      (bind _returnvalue (`|SpawnActorFromClass` (`|GetArrayItem` _spawnables _index) (`KismetMathLibrary.MakeTransform` (`SplineComponent.GetLocationAtDistanceAlongSpline` _spline _currentsplinedistance "World") (`SplineComponent.GetRotationAtDistanceAlongSpline` _spline _currentsplinedistance "World")) "Undefined" "OverrideRootScale" null null))
      (set `/Game/Blueprints/ShoppingCarts.SplineReference` (`local.CurrentSpline`) _returnvalue)
      (set `/Game/Blueprints/ShoppingCarts.Distance` (`local.CurrentSplineDistance`) _returnvalue)
      (`Pawn.SpawnDefaultController` _returnvalue)
      (set `local.CurrentSplineDistance` (+ (`local.CurrentSplineDistance`) (`local.Division`)))
      (if (>= _index (- (`KismetArrayLibrary.Array_Length` _spawnables) 1))
        (set `local.Index` 0)
        (else
          (`/Engine/EditorBlueprintResources/StandardMacros.IncrementInt` (`local.Index`)))))
    (set `local.CurrentSplineDistance` 0.0)))

(fn `UserConstructionScript`)