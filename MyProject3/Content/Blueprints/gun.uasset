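; A grabbable VR gun Actor that fires projectiles while held, picked up through BP_MotionController.
; Pickup turns off physics on the Cube and attaches the root to the given component, while Drop detaches the Actor and restores physics.
; Both set a Grabbed flag that gates the trigger input, which calls PewPew to spawn a Projectile just ahead of the Arrow component and print a debug string.
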(event `/Game/VirtualRealityBP/Blueprints/PickupActorInterface.Pickup`
  (params (AttachTo :type "SceneComponent Object Reference"))
  (`PrimitiveComponent.SetSimulatePhysics` (`self.Cube`) false)
  (`SceneComponent.K2_AttachToComponent` (`self.K2_GetRootComponent`) AttachTo "None" "KeepWorld" "KeepWorld" "KeepWorld" false)
  (set `self.Grabbed` true))

(event `/Game/VirtualRealityBP/Blueprints/PickupActorInterface.Drop`
  (`PrimitiveComponent.SetSimulatePhysics` (`self.Cube`) true)
  (`self.K2_DetachFromActor` "KeepWorld" "KeepWorld" "KeepWorld")
  (set `self.Grabbed` false))

(event `InputAction|trigger`
  (params (Key :type "Key Structure"))
  (:`Pressed`
    (if (`self.Grabbed`)
      (`self.PewPew`))))

(event `PewPew`
  (bind _arrow (`self.Arrow`))
  (`|SpawnActorFromClass` "/Game/Blueprints/Projectile.Projectile_C" (`KismetMathLibrary.MakeTransform` (+ (`SceneComponent.K2_GetComponentLocation` _arrow) (`KismetMathLibrary.GetForwardVector` (`SceneComponent.K2_GetComponentRotation` _arrow)))) "Undefined" "OverrideRootScale" null null)
  (`KismetSystemLibrary.PrintString` "pew"))

(fn `UserConstructionScript`)