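; Projectile actor that knocks physics props around and blasts Appleheads targets.
; On a hit with a physics-simulating component, it applies an impulse scaled from its velocity at its own location, then destroys itself.
; Its Sphere overlap casts the other actor to Appleheads, calls Blasted on it and destroys that actor, leaving the projectile alive.
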(event `self.ReceiveHit`
  (params (MyComp :type "PrimitiveComponent Object Reference") (Other :type "Actor Object Reference") (OtherComp :type "PrimitiveComponent Object Reference") (bSelfMoved :type Boolean) (HitLocation :type "Vector Structure") (HitNormal :type "Vector Structure") (NormalImpulse :type "Vector Structure") (Hit :type "HitResult Structure (by ref)"))
  ;[1 1 1] If a prop is shot the project will effect it.
  (if (`SceneComponent.IsSimulatingPhysics` OtherComp "None")
    (`PrimitiveComponent.AddImpulseAtLocation` OtherComp (* (`self.GetVelocity`) 100.0) (`self.K2_GetActorLocation`) "None")
    (`self.K2_DestroyActor`)))

(event `self.Sphere.OnComponentBeginOverlap`
  (params (OverlappedComponent :type "PrimitiveComponent Object Reference") (OtherActor :type "Actor Object Reference") (OtherComp :type "PrimitiveComponent Object Reference") (OtherBodyIndex :type Integer) (bFromSweep :type Boolean) (SweepResult :type "HitResult Structure (by ref)"))
  ;[1 1 1] Destroys apple after it's hit
  (bind _asappleheads (cast `/Game/Blueprints/Appleheads` OtherActor))
  (`/Game/Blueprints/Appleheads.Blasted` _asappleheads)
  (`self.K2_DestroyActor` _asappleheads))

(fn `UserConstructionScript`)