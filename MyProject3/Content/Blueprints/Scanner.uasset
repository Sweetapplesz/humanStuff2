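; Scanner Blueprint with an overlap box that scans Scannables actors entering it, like a barcode scanner.
; On overlap, a Scannable flagged Reset reloads Level1.
; Any other Scannable is marked as scanned, its point value is copied into CurrentPointsValue, and a barcode beep plays at its location.
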(event `self.Box.OnComponentBeginOverlap`
  (params (OverlappedComponent :type "PrimitiveComponent Object Reference") (OtherActor :type "Actor Object Reference") (OtherComp :type "PrimitiveComponent Object Reference") (OtherBodyIndex :type Integer) (bFromSweep :type Boolean) (SweepResult :type "HitResult Structure (by ref)"))
  ;[1 1 1] Scanning stuff
  (bind _asscannables (cast `/Game/Blueprints/Scannables` OtherActor))
  (if (`/Game/Blueprints/Scannables.Reset` _asscannables)
    (`GameplayStatics.OpenLevel` "Level1")
    (else
      (set `/Game/Blueprints/Scannables.IsScanned` true _asscannables)
      (set `self.currentPointsValue` (`/Game/Blueprints/Scannables.Pointsvalue` _asscannables))
      (`GameplayStatics.PlaySoundAtLocation` "/Game/Audio/se_barcodeBeep__1_.se_barcodeBeep__1_" (`self.K2_GetActorLocation` _asscannables) (struct) 1.0 1.0 0.0 null null null))))

(fn `UserConstructionScript`)