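; BabyCarts is a cart actor that rides along a referenced spline, resetting its distance to zero near the spline's end so it loops.
; BeginPlay randomly picks a yellow or red material and a points target, caches the first TriggerBox found as CartPoint, and reveals its skeletal mesh after a delay.
; Tick calls LocationUpdate and Movement.
; AddAlien only sets a visibility flag; hide and alien-voice fragments are left unwired.
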(event `self.ReceiveBeginPlay`
  (`parent.ReceiveBeginPlay`)
  (`|ExecutionSequence`
    (:`then_0`
      ;[1 1 1] Set Color
      (set `self.NewVar_0` (`KismetMathLibrary.RandomIntegerInRange` 0 1))
      (if (== (`self.NewVar_0`) 0)
        (set `self.Color` "Yellow")
        (bind _output_get (set `self.Color2` (`|GetArrayItem` (`self.Material`))))
        (`PrimitiveComponent.SetMaterial` (`self.StaticMesh`) 0 _output_get)
        (else
          (set `self.Color` "Red")
          (bind _output_get_2 (set `self.Color2` (`|GetArrayItem` (`self.Material`) 1)))
          (`PrimitiveComponent.SetMaterial` (`self.StaticMesh`) 0 _output_get_2))))
    (:`then_1`
      (set `self.PointsNeeded` (`KismetMathLibrary.RandomIntegerInRange` 10 40))
      (bind _outactors (`GameplayStatics.GetAllActorsOfClass` "/Script/Engine.TriggerBox"))
      (set `self.CartPoint` (`|GetArrayItem` _outactors)))
    (:`then_2`
      (`KismetSystemLibrary.Delay` 5.0)
      (`SceneComponent.SetVisibility` (`self.SkeletalMesh`) true false))))

(event `self.ReceiveTick`
  (params (DeltaSeconds :type "Float (single-precision)"))
  ;[1 1 1] Move on spline
  (`self.Location_Update`)
  (`self.Movement`)
  (if (`KismetMathLibrary.NearlyEqual_FloatFloat` (`self.Distance`) (`SplineComponent.GetSplineLength` (`/Game/Blueprints/CartSpline.Spline` (`self.SplineReference`))) 10.0)
    (set `self.Distance` 0.0)))

(event `AddAlien`
  (set `self.Vis` true))

(fn `UserConstructionScript`
  (`parent.UserConstructionScript`))