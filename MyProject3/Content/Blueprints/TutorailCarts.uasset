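; Tutorial shopping cart that scores points from Scannables overlapping its box, destroying itself after a short delay once the required points are reached.
; Scanned items add their value, call their Scanned function and trigger confetti and sound; unscanned ones only print a message.
; Movement is inactive: spline-following helper functions are never called, the Move event is empty, and the random AI roaming, rotation and timeline logic is disconnected.
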(event `self.Box.OnComponentBeginOverlap`
  (params (OverlappedComponent :type "PrimitiveComponent Object Reference") (OtherActor :type "Actor Object Reference") (OtherComp :type "PrimitiveComponent Object Reference") (OtherBodyIndex :type Integer) (bFromSweep :type Boolean) (SweepResult :type "HitResult Structure (by ref)"))
  ;[1 1 1] Point Check
  (bind _asscannables (cast `/Game/Blueprints/Scannables` OtherActor))
  (if (`/Game/Blueprints/Scannables.IsScanned` _asscannables)
    (`ActorComponent.Activate` (`self.confetti`) false)
    (`KismetSystemLibrary.PrintString` "MMMM TASTY!")
    (bind _output_get (set `self.Points` (+ (`self.Points`) (`/Game/Blueprints/Scannables.Pointsvalue` _asscannables))))
    (`KismetSystemLibrary.PrintString` "Hello")
    (`/Game/Blueprints/Scannables.Scanned` _asscannables)
    (`GameplayStatics.PlaySoundAtLocation` "/Game/Audio/Pixel_Noise4_by_abbasgamez.Pixel_Noise4_by_abbasgamez" (`self.K2_GetActorLocation`) (struct) 1.0 1.0 0.0 null null null)
    (if (>= _output_get (`self.PointsNeeded`))
      (`KismetSystemLibrary.Delay` 2.0)
      (`self.K2_DestroyActor`)
      (`KismetSystemLibrary.PrintString` "Aw fuck"))
    (else
      (`KismetSystemLibrary.PrintString` "I aint no theif"))))

(event `self.ReceiveBeginPlay`
  (set `self.Speed` (`self.Movespeed`)))

(event `Move`
  ;[1 1 1] Move
)

(fn `Location_Update`
  (bind (_returnvalue_x _returnvalue_y _returnvalue_z) (`KismetMathLibrary.BreakVector` (`self.K2_GetActorLocation`)))
  (bind _splinereference (`self.SplineReference`))
  (bind (_returnvalue_x_2 _returnvalue_y_2) (`KismetMathLibrary.BreakVector` (`SplineComponent.GetLocationAtDistanceAlongSpline` (`/Game/Blueprints/CartSpline.Spline` _splinereference) (`self.Distance`) "World")))
  (`self.K2_SetActorLocationAndRotation` (`KismetMathLibrary.MakeVector` _returnvalue_x_2 _returnvalue_y_2 _returnvalue_z) (`SplineComponent.GetRotationAtDistanceAlongSpline` (`/Game/Blueprints/CartSpline.Spline` _splinereference) (`self.Distance`) "World")))

(fn `Movement`
  (bind _returnvalue (* (`self.Speed`) (`self.AxisValue`)))
  (set `self.Accel` _returnvalue)
  (set `self.Distance` (+ (`self.Distance`) (* _returnvalue (`GameplayStatics.GetWorldDeltaSeconds`)))))

(fn `UserConstructionScript`)