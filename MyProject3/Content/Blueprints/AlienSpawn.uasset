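; AlienSpawn is a placed spawner actor that periodically creates Aliens actors at its own location.
; BeginPlay starts a looping timer that calls SpawnAlien every fifteen seconds, which spawns an alien from the actor's position alone.
; Leftover disconnected nodes, including pawn and Timer casts, a time-limit check and a delay, never run.
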(event `self.ReceiveBeginPlay`
  (`KismetSystemLibrary.K2_SetTimer` null "SpawnAlien" 15.0 true))

(event `SpawnAlien`
  (`|SpawnActorFromClass` "/Game/Blueprints/Aliens.Aliens_C" (`KismetMathLibrary.Conv_VectorToTransform` (`self.K2_GetActorLocation`)) "Undefined" "OverrideRootScale" null null))

(fn `UserConstructionScript`)