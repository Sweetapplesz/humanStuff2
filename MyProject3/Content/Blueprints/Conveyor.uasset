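; Conveyor belt actor that carries Scannables along its forward direction, in a game using a MotionControllerPawn.
; Box overlap flags an ungrabbed item as having hit the conveyor and, if its Phy flag is set, offsets overlapping Scannables by a Speed-scaled vector.
; A zero-length Delay loops back through the checks to repeat the push without Tick.
; Each overlap also raises Speed slightly once player Points reach a threshold.
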(event `self.Box.OnComponentBeginOverlap`
  (params (OverlappedComponent :type "PrimitiveComponent Object Reference") (OtherActor :type "Actor Object Reference") (OtherComp :type "PrimitiveComponent Object Reference") (OtherBodyIndex :type Integer) (bFromSweep :type Boolean) (SweepResult :type "HitResult Structure (by ref)"))
  (`|ExecutionSequence`
    (:`then_0`
      (bind _asscannables (cast `/Game/Blueprints/Scannables` OtherActor :!label _label))
      (`/Engine/EditorBlueprintResources/StandardMacros.IsValid` "/Game/Blueprints/Scannables.Scannables"
        (:`Is Valid`
          (if (not (`/Game/Blueprints/Scannables.Grabbed` _asscannables))
            (set `/Game/Blueprints/Scannables.Hitconveyor` true _asscannables)
            (if (`/Game/Blueprints/Scannables.Phy` _asscannables)
              ;[1 1 1] Pushes forward
              (for _array_element (`PrimitiveComponent.GetOverlappingActors` (`self.Box`) "/Game/Blueprints/Scannables.Scannables_C")
                (set `self.Push` (* (`KismetMathLibrary.GetForwardVector` (`self.K2_GetActorRotation`)) (* (`self.Speed`) 0.1)))
                (`self.K2_AddActorWorldOffset` _array_element (`self.Push`) false false)
                (`KismetSystemLibrary.Delay` 0.0)
                (goto _label)))))))
    (:`then_1`
      ;[1 1 1] Speed up
      (bind _asmotion_controller_pawn (cast `/Game/VirtualRealityBP/Blueprints/MotionControllerPawn` (`GameplayStatics.GetPlayerPawn` 0)))
      (if (>= (`/Game/VirtualRealityBP/Blueprints/MotionControllerPawn.Points` _asmotion_controller_pawn) 150)
        (set `self.Speed` (+ (`self.Speed`) 0.1))
        (`/Engine/EditorBlueprintResources/StandardMacros.IsValid` "/Game/Blueprints/Scannables.Scannables")))))

(fn `UserConstructionScript`)