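; Walker actor that travels along the spline of a referenced Walkerspline, looping back to the start at the end.
; Each tick it snaps X, Y and rotation to the spline at the current distance, keeping its own Z height.
; It then advances that distance by Speed times Axis and delta time, resetting to zero within a small tolerance of the spline length.
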(event `self.ReceiveTick`
  (params (DeltaSeconds :type "Float (single-precision)"))
  ;[1 1 1] Move on spline
  (`self.LocationUpdate`)
  (`self.Movement`)
  (if (`KismetMathLibrary.NearlyEqual_FloatFloat` (`self.dis`) (`SplineComponent.GetSplineLength` (`/Game/Blueprints/WalkerSpline.Spline` (`self.Walkerspline`))) 10.0)
    (set `self.dis` 0.0)))

(fn `lOCATIONUPDATE`
  (bind (_returnvalue_x _returnvalue_y _returnvalue_z) (`KismetMathLibrary.BreakVector` (`self.K2_GetActorLocation`)))
  (bind _walkerspline (`self.Walkerspline`))
  (bind _dis (`self.Dis`))
  (bind (_returnvalue_x_2 _returnvalue_y_2) (`KismetMathLibrary.BreakVector` (`SplineComponent.GetLocationAtDistanceAlongSpline` (`/Game/Blueprints/WalkerSpline.Spline` _walkerspline) _dis "World")))
  (`self.K2_SetActorLocationAndRotation` (`KismetMathLibrary.MakeVector` _returnvalue_x_2 _returnvalue_y_2 _returnvalue_z) (`SplineComponent.GetRotationAtDistanceAlongSpline` (`/Game/Blueprints/WalkerSpline.Spline` _walkerspline) _dis "World")))

(fn `mOvement`
  (bind _returnvalue (* (`self.Speed`) (`self.Axis`)))
  (set `self.Accel` _returnvalue)
  (set `self.dis` (+ (`self.dis`) (* _returnvalue (`GameplayStatics.GetWorldDeltaSeconds`)))))

(fn `UserConstructionScript`)